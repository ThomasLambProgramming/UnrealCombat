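; Player character Blueprint that owns the HUD, creating the crosshair and player health widgets on BeginPlay.
; OnPlayerHit refreshes the HP text and progress bar from the current and max health getters.
; OnChangeScrollSelected highlights one of five crosshair slots in red by scroll index, resetting the previously cached slot to white.
; Cannon attack start and end events are empty stubs, and the construction script does nothing.
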(event EventBeginPlay
  (bind _returnvalue (UserInterface|CreateWidget "/Game/Blueprints/Widgets/WB_Crosshair.WB_Crosshair_C"))
  (UserInterface|Viewport|AddtoViewport _returnvalue 0)
  (bind _output_get (Variables|Default|SetCrossHair _returnvalue))
  (bind _output_get_2 (Variables|Default|SetPreviousActiveSlotUI (Variables|/Game/Blueprints/Widgets/WB_Crosshair.WB_Crosshair_C|GetSlot1 _output_get)))
  (Appearance|SetColorandOpacity _output_get_2 (Class|KismetMathLibrary|LinearColorRed) :!class /Script/UMG.Image)
  (bind _returnvalue_2 (UserInterface|CreateWidget "/Game/Blueprints/Widgets/WB_PlayerHealth.WB_PlayerHealth_C"))
  (UserInterface|Viewport|AddtoViewport _returnvalue_2 0)
  (Variables|Default|SetPlayerHealthUI _returnvalue_2))

(event EventOnPlayerHit
  (params (DamageAmount :type Float%20%28single-precision%29) (ActorThatAttacked :type Actor%20Object%20Reference))
  (Variables|/Script/UMG.TextBlock|SetText (Variables|/Game/Blueprints/Widgets/WB_PlayerHealth.WB_PlayerHealth_C|GetHealthBarText (Variables|Default|GetPlayerHealthUI)) (Utilities|Text|ToText(String) (Utilities|String|Append (Utilities|String|Append (Utilities|String|Append "HP " (Utilities|String|ToString(Integer) (Class|KismetMathLibrary|ToInt64(Float) (Class|PlayerCharacter|GetCurrentPlayerHealth)))) " / ") (Utilities|String|ToString(Integer) (Class|KismetMathLibrary|ToInt64(Float) (Class|PlayerCharacter|GetMaxPlayerHealth))))))
  (Progress|SetPercent (Variables|/Game/Blueprints/Widgets/WB_PlayerHealth.WB_PlayerHealth_C|GetHealthProgressBar (Variables|Default|GetPlayerHealthUI)) (/ (Class|PlayerCharacter|GetCurrentPlayerHealth) (Class|PlayerCharacter|GetMaxPlayerHealth))))

(event EventOnCannonAttackStarted)

(event EventOnCannonAttackEnded)

(event EventOnChangeScrollSelected
  (params (scrollIndex :type Integer))
  (Appearance|SetColorandOpacity (Variables|Default|GetPreviousActiveSlotUI) (Class|KismetMathLibrary|LinearColorWhite) :!class /Script/UMG.Image)
  (bind _output_get (Variables|Default|SetPreviousActiveSlotUI (Utilities|Select :Index scrollIndex :Option%200 (Variables|/Game/Blueprints/Widgets/WB_Crosshair.WB_Crosshair_C|GetSlot1 (Variables|Default|GetCrossHair)) :Option%201 (Variables|/Game/Blueprints/Widgets/WB_Crosshair.WB_Crosshair_C|GetSlot2 (Variables|Default|GetCrossHair)) :Option%202 (Variables|/Game/Blueprints/Widgets/WB_Crosshair.WB_Crosshair_C|GetSlot3 (Variables|Default|GetCrossHair)) :Option%203 (Variables|/Game/Blueprints/Widgets/WB_Crosshair.WB_Crosshair_C|GetSlot4 (Variables|Default|GetCrossHair)) :Option%204 (Variables|/Game/Blueprints/Widgets/WB_Crosshair.WB_Crosshair_C|GetSlot5 (Variables|Default|GetCrossHair)))))
  (Appearance|SetColorandOpacity _output_get (Class|KismetMathLibrary|LinearColorRed) :!class /Script/UMG.Image))

(fn ConstructionScript)