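; Behavior tree service for the vampire enemy that keeps the chase-related blackboard keys updated.
; On activation it stores the first BP_ThirdPersonCharacter found as the player key.
; Each tick it copies the player-in-vision flag from BP_EnemyController to the blackboard.
; It writes the controller's last known player location only when that flag differs from the previous tick's cached value.
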(event EventReceiveActivationAI
  (params (OwnerController :type AI%20Controller%20Object%20Reference) (ControlledPawn :type Pawn%20Object%20Reference))
  (bind _outactors (Actor|GetAllActorsOfClass "/Game/Blueprints/ParentAssets/BP_ThirdPersonCharacter.BP_ThirdPersonCharacter_C"))
  (Class|BTFunctionLibrary|SetBlackboardValueasObject (Variables|Default|GetPlayerKey) (Utilities|Array|Get(acopy) _outactors)))

(event EventReceiveTickAI
  (params (OwnerController :type AI%20Controller%20Object%20Reference) (ControlledPawn :type Pawn%20Object%20Reference) (DeltaSeconds :type Float%20%28single-precision%29))
  (bind _asbp_enemy_controller (Utilities|Casting|CastToBP_EnemyController OwnerController))
  (Class|BTFunctionLibrary|SetBlackboardValueasBool (Variables|Default|GetCanSeePlayer) (Variables|/Game/Blueprints/Enemy_Vampire/BP_EnemyController.BP_EnemyController_C|GetPlayerInVision _asbp_enemy_controller))
  (if (== (Variables|/Game/Blueprints/Enemy_Vampire/BP_EnemyController.BP_EnemyController_C|GetPlayerInVision _asbp_enemy_controller) (Variables|Default|GetLastCanSeePlayer))
    _
    (else
      (AI|BehaviorTree|SetBlackboardValueasVector (Variables|Default|GetLastKnownPositionKey) (Variables|/Game/Blueprints/Enemy_Vampire/BP_EnemyController.BP_EnemyController_C|GetLastKnownPlayerLocation _asbp_enemy_controller))))
  (Variables|Default|SetLastCanSeePlayer (Class|BTFunctionLibrary|GetBlackboardValueasBool (Variables|Default|GetCanSeePlayer))))