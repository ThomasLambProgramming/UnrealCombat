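; BP_StandardAi is an AI Blueprint that displays its health and latest damage through widget components.
; On BeginPlay it fills the health bar, binds to the AI health-changed delegate and seeds the damage number text with max health.
; Each health change updates the bar to the current fraction and shows the absolute difference from the cached previous health, so healing also appears as a positive number.
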(event Custom|OnAiHealthChangedDelegate_Event
  (Progress|SetPercent (Variables|Default|GetHealthProgressBarComponent) (/ (Variables|Default|GetCurrentHealth) (Variables|Default|GetMaxHealth)))
  (bind _aswb_damage_number (Utilities|Casting|CastToWB_DamageNumber (UserInterface|GetWidget (Variables|Default|GetDamageNumber))))
  (Rendering|Components|TextRender|SetText (Variables|/Game/Blueprints/WB_DamageNumber.WB_DamageNumber_C|GetTextBlock_69 _aswb_damage_number) (Utilities|Text|ToText(Float) (Math|Float|Absolute(Float) (- (Variables|Default|GetPreviousHealth) (Variables|Default|GetCurrentHealth))) "HalfToEven"))
  (Variables|Default|SetPreviousHealth (Variables|Default|GetCurrentHealth)))

(event EventBeginPlay
  (bind _aswb_enemy_health (Utilities|Casting|CastToWB_EnemyHealth (UserInterface|GetWidget (Variables|Default|GetHealthBar))))
  (bind _output_get (Variables|Default|SetHealthProgressBarComponent (Variables|/Game/Blueprints/WB_EnemyHealth.WB_EnemyHealth_C|GetProgressBarComp _aswb_enemy_health)))
  (Progress|SetPercent _output_get 1.0)
  (EventDispatchers|BindEventtoOnAiHealthChangedDelegate (EventDispatchers|CreateEvent :!event Custom|OnAiHealthChangedDelegate_Event))
  (Variables|Default|SetPreviousHealth (Variables|Default|GetMaxHealth))
  (bind _aswb_damage_number (Utilities|Casting|CastToWB_DamageNumber (UserInterface|GetWidget (Variables|Default|GetDamageNumber))))
  (Rendering|Components|TextRender|SetText (Variables|/Game/Blueprints/WB_DamageNumber.WB_DamageNumber_C|GetTextBlock_69 _aswb_damage_number) (Utilities|Text|ToText(Float) (Variables|Default|GetPreviousHealth) "HalfToEven")))

(fn ConstructionScript)