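; Test actor that builds a staircase of cubes by spawning copies of itself, each offset from the tracked top block.
; While SpawnMoreCubes is set, a briefly delayed Tick initializes CurrentTopBlock to self or spawns the next copy when self is that block.
; Key 1 spawns a copy manually and key 2 destroys the tracked block.
; The construction script assigns the cube mesh and prints a debug string.
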(event EventBeginPlay)

(event Collision|EventActorBeginOverlap
  (params (OtherActor :type Actor%20Object%20Reference)))

(event EventTick
  (params (DeltaSeconds :type Float%20%28single-precision%29))
  (if (Variables|Default|GetSpawnMoreCubes)
    (Utilities|FlowControl|Delay 0.01)
    (if (!= self (Variables|Default|GetCurrentTopBlock))
      (Utilities|IsValid (Variables|Default|GetCurrentTopBlock)
        (:Is%20Not%20Valid
          (Variables|Default|SetCurrentTopBlock self)))
      (else
        (bind _returnvalue (Game|SpawnActorfromClass "BP_Testing_C" (Math|Transform|MakeTransform (+ (.location (Transformation|GetActorTransform (Variables|Default|GetCurrentTopBlock))) "0.000000,-100.000000,100.000000") (.rotation (Transformation|GetActorTransform (Variables|Default|GetCurrentTopBlock))) (.scale (Transformation|GetActorTransform (Variables|Default|GetCurrentTopBlock)))) "Undefined" "MultiplyWithRoot" 0 0))
        (Variables|Default|SetCurrentTopBlock _returnvalue)))))

(event Input|KeyboardEvents|1
  (params (Key :type Key%20Structure))
  (:Pressed
    (bind _returnvalue (Game|SpawnActorfromClass "BP_Testing_C" (Math|Transform|MakeTransform (+ (.location (Transformation|GetActorTransform (Variables|Default|GetCurrentTopBlock))) "0.000000,-100.000000,100.000000") (.rotation (Transformation|GetActorTransform (Variables|Default|GetCurrentTopBlock))) (.scale (Transformation|GetActorTransform (Variables|Default|GetCurrentTopBlock)))) "Undefined" "MultiplyWithRoot" 0 0))
    (Variables|Default|SetCurrentTopBlock _returnvalue)))

(event Input|KeyboardEvents|2
  (params (Key :type Key%20Structure))
  (bind _currenttopblock (Variables|Default|GetCurrentTopBlock))
  (:Pressed
    (Utilities|IsValid _currenttopblock
      (:Is%20Valid
        (Actor|DestroyActor _currenttopblock)))))

(fn ConstructionScript
  (Components|StaticMesh|SetStaticMesh (Variables|Default|GetCuabe) (Variables|Default|GetStaticMeshExample))
  (Development|PrintString "Hello"))

(fn Func)